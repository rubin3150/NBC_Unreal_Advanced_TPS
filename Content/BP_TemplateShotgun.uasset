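; Shotgun weapon template Blueprint that overrides firing from a parent class, which supplies Fire and Reload.
; Left click calls Fire and prints the ammo count; R prints a reload message and, like the Reload event, calls the parent's Reload.
; ProcessFiring casts several Visibility line traces in a random cone from FirePoint with debug drawing, applying DamagePerHit to each hit actor.
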(event EventReload
  ;[0.15 0.15 0.15 0.5] 블루프린트 부모만 작동
  (|CallParentFunction))

(event EventProcessFiring
  (bind _firepoint (Variables|Default|GetFirePoint))
  (bind _returnvalue (Transformation|GetWorldLocation _firepoint))
  ;[0.15 0.15 0.15 0.5] Fire
  (for _index (range 1 4)
    (bind (_outhit _returnvalue_2) (Collision|LineTraceByChannel _returnvalue (+ _returnvalue (* (Math|Random|RandomUnitVectorinConeinDegrees (Math|Vector|GetForwardVector _firepoint) 2e+01) (Variables|Default|GetRange))) "TraceTypeQuery1" false (Utilities|Array|MakeArray (Components|GetOwner)) "ForDuration"))
    (if _returnvalue_2
      (Game|Damage|ApplyDamage (.HitActor (Collision|BreakHitResult _outhit)) (Variables|Default|GetDamagePerHit) 0 0))))

(event EventBeginPlay
  (Utilities|FlowControl|Delay 0.1))

(event Input|MouseEvents|LeftMouseButton
  (params (Key :type Key%20Structure :default "None"))
  (:Pressed
    (Class|WeaponBase|Fire)
    (Development|PrintString (Utilities|String|Append (Utilities|String|ToString(Integer) (Variables|Default|GetCurrentAmmo)) "/" (Utilities|String|ToString(Integer) (Variables|Default|GetMaxAmmo))) true true "(R=0.000000,G=1.000000,B=0.000000,A=1.000000)")))

(event Input|KeyboardEvents|R
  (params (Key :type Key%20Structure :default "None"))
  (:Pressed
    (Development|PrintString "재장전 되었습니다.")
    ;[0.15 0.15 0.15 0.5] 블루프린트 부모만 작동
    (|CallParentFunction)))

(fn ConstructionScript)